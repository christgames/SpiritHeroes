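; Enemy monster that chases and fights the player, with health and battle state kept in the Globals game instance.
; In battle mode, pawn sensing starts an AI move to the player, dealing damage on arrival if MonsterFire is set.
; Sword hits and delayed head or body contact apply damage, with head contact flagging a headshot.
; Helpers play random hurt sounds, gendered by active player, and custom events toggle the monster on or off.
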(event OnComponentBeginOverlap(Head)
  (params (OverlappedComponent :type Primitive%20Component%20Object%20Reference) (OtherActor :type Actor%20Object%20Reference) (OtherComp :type Primitive%20Component%20Object%20Reference) (OtherBodyIndex :type Integer) (bFromSweep :type Boolean) (SweepResult :type Hit%20Result%20Structure%20%28by%20ref%29))
  ;[1 1 1] Player Touches Monster (Head)
  (Utilities|Casting|CastToPlayer OtherActor)
  (Utilities|FlowControl|Delay 0.5)
  (bind _asglobals (Utilities|Casting|CastToGlobals (Game|GetGameInstance)))
  (Audio|PlaySound2D "/Game/Sounds/boink.boink")
  (CallFunction|MonsterOuchSound)
  (Variables|/Game/Globals.Globals_C|SetMonsterHealth _asglobals (- (Variables|/Game/Globals.Globals_C|GetMonsterHealth _asglobals) 5))
  (Variables|/Game/Globals.Globals_C|SetHeadShot _asglobals true))

(event OnComponentBeginOverlap(Body)
  (params (OverlappedComponent :type Primitive%20Component%20Object%20Reference) (OtherActor :type Actor%20Object%20Reference) (OtherComp :type Primitive%20Component%20Object%20Reference) (OtherBodyIndex :type Integer) (bFromSweep :type Boolean) (SweepResult :type Hit%20Result%20Structure%20%28by%20ref%29))
  ;[1 1 1] Player Touches Monster (Body)
  (Utilities|Casting|CastToPlayer OtherActor)
  (Utilities|FlowControl|Delay 0.5)
  (bind _asglobals (Utilities|Casting|CastToGlobals (Game|GetGameInstance)))
  (Variables|/Game/Globals.Globals_C|SetPlayerHealth _asglobals (- (Variables|/Game/Globals.Globals_C|GetPlayerHealth _asglobals) 10))
  (Variables|/Game/Globals.Globals_C|SetMonsterHealth _asglobals (- (Variables|/Game/Globals.Globals_C|GetMonsterHealth _asglobals) 5))
  (CallFunction|PlayerOuchSound))

(event OnSeePawn(MonsterSensing)
  (params (Pawn :type Pawn%20Object%20Reference))
  ;[1 1 1] Monster Sees Player
  (bind _asglobals (Utilities|Casting|CastToGlobals (Game|GetGameInstance)))
  (if (Variables|/Game/Globals.Globals_C|GetBattleMode _asglobals)
    (bind _asplayer (Utilities|Casting|CastToPlayer Pawn))
    (AI|AIMoveTo self "0, 0, 0" _asplayer 5.0 true
      (:then
        (bind _asglobals_2 (Utilities|Casting|CastToGlobals (Game|GetGameInstance)))
        (if (Variables|/Game/Globals.Globals_C|GetMonsterFire _asglobals_2)
          (Variables|/Game/Globals.Globals_C|SetMonsterFire _asglobals_2 false)
          (Variables|/Game/Globals.Globals_C|SetPlayerHealth _asglobals_2 (- (Variables|/Game/Globals.Globals_C|GetPlayerHealth _asglobals_2) 10))
          (CallFunction|PlayerOuchSound))))))

(event Custom|DisableMonster
  ;[1 1 1] Disable Monster
  (Rendering|SetActorHiddenInGame true)
  (Actor|Tick|SetActorTickEnabled false)
  (Collision|SetActorEnableCollision false))

(event Custom|EnableMonster
  ;[1 1 1] Enable Monster
  (Rendering|SetActorHiddenInGame false)
  (Actor|Tick|SetActorTickEnabled true)
  (Collision|SetActorEnableCollision true))

(event Collision|EventActorBeginOverlap
  (params (OtherActor :type Actor%20Object%20Reference))
  ;[1 1 1] Weapon Hit Monster
  (if (== (Utilities|GetClass OtherActor) "/Game/Blueprints/Sword.Sword_C")
    (bind _asglobals (Utilities|Casting|CastToGlobals (Game|GetGameInstance)))
    (Variables|/Game/Globals.Globals_C|SetMonsterHealth _asglobals (- (Variables|/Game/Globals.Globals_C|GetMonsterHealth _asglobals) 1))
    (CallFunction|MonsterOuchSound)
    (Audio|PlaySound2D "/Game/Sounds/sword.sword")))

(fn ConstructionScript)

(fn PlayerOuchSound
  ;[1 1 1] Player Ouch Sound
  (bind _asglobals (Utilities|Casting|CastToGlobals (Game|GetGameInstance)))
  (switch int (Variables|/Game/Globals.Globals_C|GetActivePlayer _asglobals)
    (:0
      (switch int (Math|Random|RandomIntegerinRange 0 1) :!label _label
        (:0
          (Audio|PlaySound2D "/Game/Voices/ouch1-girl.ouch1-girl"))
        (:1
          (Audio|PlaySound2D "/Game/Voices/ouch2-girl.ouch2-girl"))))
    (:1
      (switch int (Math|Random|RandomIntegerinRange 0 1) :!label _label_2
        (:0
          (Audio|PlaySound2D "/Game/Sounds/ouch1-boy.ouch1-boy"))
        (:1
          (Audio|PlaySound2D "/Game/Sounds/ouch2-boy.ouch2-boy"))))
    (:2
      (goto _label))
    (:3
      (goto _label_2))
    (:4
      (goto _label))
    (:5
      (goto _label_2))))

(fn MonsterOuchSound
  ;[1 1 1] Monster Ouch Sound
  (switch int (Math|Random|RandomIntegerinRange 0 4)
    (:0
      (Audio|PlaySound2D "/Game/Voices/monsterfight1.monsterfight1"))
    (:1
      (Audio|PlaySound2D "/Game/Voices/monsterfight2.monsterfight2"))
    (:2
      (Audio|PlaySound2D "/Game/Voices/monsterfight3.monsterfight3"))
    (:3
      (Audio|PlaySound2D "/Game/Voices/monsterfight4.monsterfight4"))
    (:4
      (Audio|PlaySound2D "/Game/Voices/monsterfight5.monsterfight5"))))