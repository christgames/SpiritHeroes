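; GreenMinion is an enemy that chases the player during battle mode and reacts to sword hits.
; Pawn sensing triggers AI movement toward the seen Player when the game instance's BattleMode flag is set.
; Sword overlaps decrement MonsterHealth on the Globals game instance, then play a random ouch sound and a sword sound.
; Enable and disable events toggle its visibility, tick and collision together.
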(event OnSeePawn(GreenMinionSensing)
  (params (Pawn :type Pawn%20Object%20Reference))
  ;[1 1 1] Minion Sees Player
  (bind _asglobals (Utilities|Casting|CastToGlobals (Game|GetGameInstance)))
  (if (Variables|/Game/Globals.Globals_C|GetBattleMode _asglobals)
    (bind _asplayer (Utilities|Casting|CastToPlayer Pawn))
    (AI|AIMoveTo self "0, 0, 0" _asplayer 5.0 true)))

(event Custom|DisableGreenMinion
  ;[1 1 1] Disable Green Minion
  (Rendering|SetActorHiddenInGame true)
  (Actor|Tick|SetActorTickEnabled false)
  (Collision|SetActorEnableCollision false))

(event Custom|EnableGreenMinion
  ;[1 1 1] Enable Green Minion
  (Rendering|SetActorHiddenInGame false)
  (Actor|Tick|SetActorTickEnabled true)
  (Collision|SetActorEnableCollision true))

(event Custom|Green%20Minion%20Ouch%20Sound
  ;[1 1 1] Play Minion Ouch Sound
  (switch int (Math|Random|RandomIntegerinRange 0 5)
    (:0
      (Audio|PlaySound2D "/Game/Voices/minionfight2.minionfight2" :!label _label))
    (:1
      (goto _label))
    (:2
      (Audio|PlaySound2D "/Game/Voices/monsterfight2.monsterfight2"))
    (:3
      (Audio|PlaySound2D "/Game/Voices/monsterfight3.monsterfight3"))
    (:4
      (Audio|PlaySound2D "/Game/Voices/monsterfight4.monsterfight4"))
    (:5
      (Audio|PlaySound2D "/Game/Voices/monsterfight5.monsterfight5"))))

(event Collision|EventActorBeginOverlap
  (params (OtherActor :type Actor%20Object%20Reference))
  ;[1 1 1] Weapon Hits Minion
  (if (== (Utilities|GetClass OtherActor) "/Game/Blueprints/Sword.Sword_C")
    (bind _asglobals (Utilities|Casting|CastToGlobals (Game|GetGameInstance)))
    (Variables|/Game/Globals.Globals_C|SetMonsterHealth _asglobals (- (Variables|/Game/Globals.Globals_C|GetMonsterHealth _asglobals) 1))
    (CallFunction|GreenMinionOuchSound)
    (Audio|PlaySound2D "/Game/Sounds/sword.sword")))

(fn ConstructionScript)